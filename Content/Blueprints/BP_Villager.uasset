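; BP_Villager is a villager whose six needs (drowsiness, hunger, thirst, dirtiness, toilet, boredom) grow over time and who earns a salary.
; Tick raises each clamped need at its own rate, adds Salary when the Sky day changes, then refreshes the stats widget every frame.
; CreateStats builds that widget with the villager's icon, and bars turn red once a need reaches its threshold.
; An AIMoveTo toward the player is left unconnected.
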(event `self.ReceiveTick`
  (params (DeltaSeconds :type "Float (single-precision)"))
  (`self.UpdateStats` DeltaSeconds)
  (`self.EarnMoney`)
  (`self.Update UI`))

(fn `CreateStats`
  (returns (StatsWidget :type "/Game/Blueprints/WBP_VillagerStats Object Reference"))
  (bind _returnvalue (`|CreateWidget` "/Game/Blueprints/WBP_VillagerStats.WBP_VillagerStats_C"))
  (bind _output_get (set `self.StatsWidget` _returnvalue))
  (`Widget.SetVisibility` (`/Game/Blueprints/WBP_VillagerStats.Hot_Image` _output_get) "Hidden")
  (`Widget.SetVisibility` (`/Game/Blueprints/WBP_VillagerStats.Cold_Image` _output_get) "Hidden")
  (`Widget.SetVisibility` (`/Game/Blueprints/WBP_VillagerStats.Rain_Image` _output_get) "Hidden")
  (`Image.SetBrushFromTexture` (`/Game/Blueprints/WBP_VillagerStats.FaceIcon` _output_get) (`self.Icon`) false)
  (return _output_get))

(fn `EarnMoney`
  (if (!= (`/Game/DynamicVolumetricSky/Blueprints/BP_DynamicVolumetricSky.Days` (`self.Sky`)) (`self.LastDay`))
    (set `self.Money` (+ (`self.Money`) (`self.Salary`)))
    (set `self.LastDay` (`/Game/DynamicVolumetricSky/Blueprints/BP_DynamicVolumetricSky.Days` (`self.Sky`)))))

(fn `Update UI`
  (bind _statswidget (`self.StatsWidget`))
  (`self.UpdateProgressBar` (`/Game/Blueprints/WBP_VillagerStats.Drowzyness_Bar` _statswidget) (`self.Drowzyness`) (`self.DrowzynessThreshold`) (struct :`G` 0.129412 :`B` 1.0 :`A` 1.0))
  (`self.UpdateProgressBar` (`/Game/Blueprints/WBP_VillagerStats.Hunger_Bar` _statswidget) (`self.Hunger`) (`self.HungerThreshold`) (struct :`R` 1.0 :`G` 0.270588 :`A` 1.0))
  (`self.UpdateProgressBar` (`/Game/Blueprints/WBP_VillagerStats.Thirst_Bar` _statswidget) (`self.Thirst`) (`self.ThirstThreshold`) (struct :`R` 0.015686 :`G` 0.537255 :`B` 1.0 :`A` 1.0))
  (`self.UpdateProgressBar` (`/Game/Blueprints/WBP_VillagerStats.Dirtiness_Bar` _statswidget) (`self.Dirtiness`) (`self.DirtinessThreshold`) (struct :`R` 0.462745 :`G` 0.592157 :`B` 0.72549 :`A` 1.0))
  (`self.UpdateProgressBar` (`/Game/Blueprints/WBP_VillagerStats.Toilet_Bar` _statswidget) (`self.Toilet`) (`self.ToiletThreshold`) (struct :`R` 0.862745 :`G` 0.686275 :`B` 0.117647 :`A` 1.0))
  (`self.UpdateProgressBar` (`/Game/Blueprints/WBP_VillagerStats.Boredom_Bar` _statswidget) (`self.Boredom`) (`self.BoredomThreshold`) (struct :`R` 1.0 :`G` 0.098039 :`B` 0.541176 :`A` 1.0))
  (set `TextBlock.Text` (`KismetTextLibrary.Conv_IntToText` (`self.Money`)) (`/Game/Blueprints/WBP_VillagerStats.Money_Text` _statswidget)))

(fn `UpdateProgressBar`
  (params (ProgressBar :type "ProgressBar Object Reference") (Value :type "Float (double-precision)") (Threshold :type "Float (double-precision)") (Color :type "LinearColor Structure"))
  (bind (_drawas _tiling _mirroring _imagesize _margin _tintcolor) (break `SlateBrush` (`.FillImage` (break `ProgressBarStyle` (`ProgressBar.WidgetStyle` ProgressBar)))))
  (`ProgressBar.SetPercent` ProgressBar Value)
  (if (>= Value Threshold)
    (setmembers `SlateColor` :`StructRef` _tintcolor :`SpecifiedColor` (struct :`R` 1.0 :`G` 0.033333 :`B` 0.033333 :`A` 1.0))
    (else
      (setmembers `SlateColor` :`StructRef` _tintcolor :`SpecifiedColor` Color))))

(fn `UpdateStats`
  (params (DeltaTime :type "Float (double-precision)"))
  (set `self.Drowzyness` (`KismetMathLibrary.FClamp` (+ (* DeltaTime 0.005) (`self.Drowzyness`))))
  (set `self.Hunger` (`KismetMathLibrary.FClamp` (+ (* DeltaTime 0.01) (`self.Hunger`))))
  (set `self.Thirst` (`KismetMathLibrary.FClamp` (+ (* DeltaTime 0.015) (`self.Thirst`))))
  (set `self.Dirtiness` (`KismetMathLibrary.FClamp` (+ (* DeltaTime 0.002) (`self.Dirtiness`))))
  (set `self.Toilet` (`KismetMathLibrary.FClamp` (+ (* DeltaTime 0.015) (`self.Toilet`))))
  (set `self.Boredom` (`KismetMathLibrary.FClamp` (+ (* DeltaTime 0.02) (`self.Boredom`)))))

(fn `UserConstructionScript`)